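; Storm cloud hazard that drifts along world X by a fixed step every tick.
; Two looping timers periodically move each lightning component to a random spot on its own side of the cloud, varying Y and height.
; When a BP_Boat overlaps its box, it only prints a game-over message.
; Logic to flash the lightning's visibility exists but is never run.
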(event `self.ReceiveBeginPlay`
  (`KismetSystemLibrary.K2_SetTimerDelegate` (delegate `RandomPos 2`) 3.0 true)
  (`KismetSystemLibrary.K2_SetTimerDelegate` (delegate `RandomPos 1`) 2.0 true))

(event `RandomPos 2`
  (`SceneComponent.K2_SetRelativeLocation` (`self.Lightning_2`) (`KismetMathLibrary.MakeVector` 0.0 (`KismetMathLibrary.RandomFloatInRange` 100.0 1500.0) (`KismetMathLibrary.RandomFloatInRange` -800.0 -900.0)) false false))

(event `RandomPos 1`
  (`SceneComponent.K2_SetRelativeLocation` (`self.Lightning_1`) (`KismetMathLibrary.MakeVector` 0.0 (`KismetMathLibrary.RandomFloatInRange` -1500.0 -200.0) (`KismetMathLibrary.RandomFloatInRange` -800.0 -900.0)) false false))

(event `self.Box.OnComponentBeginOverlap`
  (params (OverlappedComponent :type "PrimitiveComponent Object Reference") (OtherActor :type "Actor Object Reference") (OtherComp :type "PrimitiveComponent Object Reference") (OtherBodyIndex :type Integer) (bFromSweep :type Boolean) (SweepResult :type "HitResult Structure (by ref)"))
  (cast `/Game/Player/Boat/BP_Boat` OtherActor)
  (`KismetSystemLibrary.PrintString` "GAME OVER!" true true (struct :`R` 1.0 :`B` 0.011103 :`A` 1.0)))

(event `self.ReceiveTick`
  (params (DeltaSeconds :type "Float (single-precision)"))
  (`self.K2_AddActorWorldOffset` (10.0 0.0 0.0)))

(fn `UserConstructionScript`)