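; BP_HubCharacter is the hub player character, able to take control of a BP_Boat it is standing in.
; Capsule begin and end overlap events with a BP_Boat set and clear an overlap flag.
; Pressing E while flagged makes player controller 0 possess the first overlapping boat, then disables the character's capsule collision, with debug prints.
; A node attaching the mesh to the boat is unconnected.
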(event `Key|E`
  (params (Key :type "Key Structure"))
  (:`Pressed`
    (if (`self.IsOverlaping`)
      (bind _asbp_boat (cast `/Game/Player/Boat/BP_Boat` (`|GetArrayItem` (`self.GetOverlappingActors` "/Game/Player/Boat/BP_Boat.BP_Boat_C"))))
      (`KismetSystemLibrary.PrintString` "true")
      (`Controller.Possess` (`GameplayStatics.GetPlayerController` 0) _asbp_boat)
      (`PrimitiveComponent.SetCollisionEnabled` (`self.CapsuleComponent`) "NoCollision")
      (else
        (`KismetSystemLibrary.PrintString` "false")))))

(event `self.CapsuleComponent.OnComponentBeginOverlap`
  (params (OverlappedComponent :type "PrimitiveComponent Object Reference") (OtherActor :type "Actor Object Reference") (OtherComp :type "PrimitiveComponent Object Reference") (OtherBodyIndex :type Integer) (bFromSweep :type Boolean) (SweepResult :type "HitResult Structure (by ref)"))
  (cast `/Game/Player/Boat/BP_Boat` OtherActor)
  (set `self.IsOverlaping` true))

(event `self.CapsuleComponent.OnComponentEndOverlap`
  (params (OverlappedComponent :type "PrimitiveComponent Object Reference") (OtherActor :type "Actor Object Reference") (OtherComp :type "PrimitiveComponent Object Reference") (OtherBodyIndex :type Integer))
  (cast `/Game/Player/Boat/BP_Boat` OtherActor)
  (set `self.IsOverlaping` false))

(fn `UserConstructionScript`)