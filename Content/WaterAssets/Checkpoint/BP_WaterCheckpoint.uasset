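; BP_WaterCheckpoint is a boat race checkpoint on the water, marked by two buoy child actors and a Niagara effect.
; While active, a BP_Boat overlapping its box prints a message, deactivates it and calls the CheckpointReached dispatcher.
; Activate enables the flag and effect.
; Deactivate clears both and swaps both buoys to a gray striped material, which Activate does not restore.
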(event `self.Box.OnComponentBeginOverlap`
  (params (OverlappedComponent :type "PrimitiveComponent Object Reference") (OtherActor :type "Actor Object Reference") (OtherComp :type "PrimitiveComponent Object Reference") (OtherBodyIndex :type Integer) (bFromSweep :type Boolean) (SweepResult :type "HitResult Structure (by ref)"))
  (if (`self.IsActive`)
    (cast `/Game/Player/Boat/BP_Boat` OtherActor)
    (`KismetSystemLibrary.PrintString` "Checkpoint!" true true (struct :`G` 1.0 :`B` 0.197003 :`A` 1.0))
    (`self.Deactivate`)
    (`self.CheckpointReached`)))

(fn `Activate`
  (set `self.IsActive` true)
  (`ActorComponent.SetActive` (`self.NS_Checkpoint`) true false))

(fn `Deactivate`
  (set `self.IsActive` false)
  (`ActorComponent.Deactivate` (`self.NS_Checkpoint`))
  (`self.GrayOutCones` (`self.BP_WaterBuoy_1`))
  (`self.GrayOutCones` (`self.BP_WaterBuoy_2`)))

(fn `GrayOutCones`
  (params (ChildCone :type "ChildActorComponent Object Reference"))
  (bind _asbp_water_buoy (cast `/Game/WaterAssets/Checkpoint/BP_WaterBuoy` (`ChildActorComponent.ChildActor` ChildCone)))
  (`PrimitiveComponent.SetMaterial` (`/Game/WaterAssets/Checkpoint/BP_WaterBuoy.Static Mesh` _asbp_water_buoy) 0 "/Game/WaterAssets/Cone/M_ConeStripedGray.M_ConeStripedGray"))

(fn `UserConstructionScript`)