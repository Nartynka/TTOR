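; Interactive portal actor that opens and closes visually as something approaches, and loads a level when the player enters it.
; The outer Box overlap activates the portal effect and scales the mesh's X and Y through a timeline, keeping Z thin.
; Leaving that Box deactivates the effect and shrinks the mesh with a second, reversed timeline.
; Overlapping Box1 with a HubCharacter opens the referenced Level.
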(event `self.Box1.OnComponentBeginOverlap`
  (params (OverlappedComponent :type "PrimitiveComponent Object Reference") (OtherActor :type "Actor Object Reference") (OtherComp :type "PrimitiveComponent Object Reference") (OtherBodyIndex :type Integer) (bFromSweep :type Boolean) (SweepResult :type "HitResult Structure (by ref)"))
  (cast `HubCharacter` OtherActor)
  (`GameplayStatics.OpenLevelBySoftObjectPtr` (`self.Level`)))

(event `self.Box.OnComponentBeginOverlap`
  (params (OverlappedComponent :type "PrimitiveComponent Object Reference") (OtherActor :type "Actor Object Reference") (OtherComp :type "PrimitiveComponent Object Reference") (OtherBodyIndex :type Integer) (bFromSweep :type Boolean) (SweepResult :type "HitResult Structure (by ref)"))
  (`ActorComponent.Activate` (`self.PortalEffect`) true)
  (bind (_direction _scale) (`Timeline|Timeline` :!via `PlayFromStart`)
    (:`Update`
      (`SceneComponent.SetWorldScale3D` (`self.PortalMesh`) (`KismetMathLibrary.MakeVector` _scale _scale 0.1)))))

(event `self.Box.OnComponentEndOverlap`
  (params (OverlappedComponent :type "PrimitiveComponent Object Reference") (OtherActor :type "Actor Object Reference") (OtherComp :type "PrimitiveComponent Object Reference") (OtherBodyIndex :type Integer))
  (`ActorComponent.Deactivate` (`self.PortalEffect`))
  (bind (_direction _scale) (`Timeline|Timeline_0` :!via `ReverseFromEnd`)
    (:`Update`
      (`SceneComponent.SetWorldScale3D` (`self.PortalMesh`) (`KismetMathLibrary.MakeVector` _scale _scale 0.1)))))

(fn `UserConstructionScript`)