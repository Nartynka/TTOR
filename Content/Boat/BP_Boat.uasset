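; Player-controlled boat pawn that drives and steers with Enhanced Input and turns the controller yaw for looking.
; Tick applies yaw from steering input and integrates throttle into a clamped Motion speed, with friction when idle, then offsets the actor along its forward vector.
; Mesh hits replace Motion with a clamped kickback scaled by its square and sign, limited by a one-second cooldown.
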(event `self.ReceiveBeginPlay`
  ;[1 1 1] Input
  (bind _asplayer_controller (cast `PlayerController` (`self.GetController`)))
  (bind _returnvalue (pcsubsystem `EnhancedInputLocalPlayerSubsystem` _asplayer_controller))
  (`/Engine/EditorBlueprintResources/StandardMacros.IsValid` _returnvalue
    (:`Is Valid`
      (`EnhancedInputSubsystemInterface.AddMappingContext` _returnvalue "/Game/Characters/Input/IMC_Default.IMC_Default" 0 (struct)))))

(event `EnhancedInput|/Game/Characters/Input/IA_Move`
  (params (ActionValue :type "Vector2D Structure") (ElapsedSeconds :type "Float (double-precision)") (TriggeredSeconds :type "Float (double-precision)") (InputAction :type "InputAction Object Reference" :default "/Game/Characters/Input/IA_Move.IA_Move"))
  ;[1 1 1] Input
  (:`Triggered`
    (set `self.Move Input` ActionValue_Y :!label _label)
    (set `self.Rotation Input` ActionValue_X))
  (:`Completed`
    (goto _label)))

(event `EnhancedInput|/Game/Characters/Input/IA_Look`
  (params (ActionValue :type "Vector2D Structure") (ElapsedSeconds :type "Float (double-precision)") (TriggeredSeconds :type "Float (double-precision)") (InputAction :type "InputAction Object Reference" :default "/Game/Characters/Input/IA_Look.IA_Look"))
  ;[1 1 1] Input
  (:`Triggered`
    (`self.AddControllerYawInput` ActionValue_X)))

(event `self.ReceiveTick`
  (params (DeltaSeconds :type "Float (single-precision)"))
  (bind (_returnvalue_x _returnvalue_y) (`KismetMathLibrary.BreakVector` (`self.GetActorForwardVector`)))
  (bind _max_speed (`self.MAX_SPEED`))
  (bind _motion (`self.Motion`))
  (bind _returnvalue (* (`self.FRICTION`) (`self.Delta Seconds`)))
  (set `self.Delta Seconds` DeltaSeconds)
  (`self.K2_AddActorWorldRotation` (`KismetMathLibrary.MakeRotator` 0.0 0.0 (`self.Rotation Input`)))
  (if (== (`self.Move Input`) 0.0)
    (set `self.Motion` (select `bool` (> (`self.Motion`) 0.0) :`false` (`KismetMathLibrary.FClamp` (+ (`self.Motion`) _returnvalue) (* (`self.MAX_SPEED`) -1.0) 0.0) :`true` (`KismetMathLibrary.FClamp` (- (`self.Motion`) _returnvalue) 0.0 (`self.MAX_SPEED`))))
    (else
      (set `self.Motion` (`KismetMathLibrary.FClamp` (+ (`self.Motion`) (* (`self.Move Input`) (`self.ACCELERATION`) (`self.Delta Seconds`))) (* -1.0 _max_speed) _max_speed))))
  (`self.K2_AddActorWorldOffset` (`KismetMathLibrary.MakeVector` (* _returnvalue_x _motion) (* _returnvalue_y _motion))))

(event `self.StaticMesh.OnComponentHit`
  (params (HitComponent :type "PrimitiveComponent Object Reference") (OtherActor :type "Actor Object Reference") (OtherComp :type "PrimitiveComponent Object Reference") (NormalImpulse :type "Vector Structure") (Hit :type "HitResult Structure (by ref)"))
  (bind _max_kickback_force (`self.Max Kickback Force`))
  ;[1 1 1] Kickback after hiting somethig
  (`/Engine/EditorBlueprintResources/StandardMacros.DoOnce` false :!label _label_2
    (:`Completed`
      (set `self.Motion` (`KismetMathLibrary.FClamp` (* (* (`self.Kickback Force Multiplyer`) (`KismetMathLibrary.SignOfFloat` (`self.Motion`))) (`KismetMathLibrary.Square` (`self.Motion`))) (* _max_kickback_force -1.0) _max_kickback_force))
      (`KismetSystemLibrary.Delay` 1.0)
      (goto _label_2 :!via `Reset`))))

(fn `UserConstructionScript`)