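; BP_Boat_2 is a player-controlled boat that constantly drives itself forward by adding force to its static mesh each Tick.
; The force follows the flattened actor forward vector scaled by Speed, which each Space press doubles with no reset.
; Enhanced Input, registered on BeginPlay, supplies steering as a per-tick yaw rotation from IA_Move and horizontal look through controller yaw from IA_Look.
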(event `self.ReceiveTick`
  (params (DeltaSeconds :type "Float (single-precision)"))
  (bind (_returnvalue_x _returnvalue_y) (`KismetMathLibrary.BreakVector` (`self.GetActorForwardVector`)))
  (`PrimitiveComponent.AddForce` (`self.StaticMesh`) (* (`KismetMathLibrary.MakeVector` _returnvalue_x _returnvalue_y) (`self.Speed`)) "None" false)
  (`self.K2_AddActorWorldRotation` (`KismetMathLibrary.MakeRotator` 0.0 0.0 (`self.Delta Rotation Z (Yaw)`))))

(event `Key|SpaceBar`
  (params (Key :type "Key Structure"))
  (:`Pressed`
    (set `self.Speed` (* (`self.Speed`) 2.0))))

(event `self.ReceiveBeginPlay`
  (bind _asplayer_controller (cast `PlayerController` (`self.GetController`)))
  (bind _returnvalue (pcsubsystem `EnhancedInputLocalPlayerSubsystem` _asplayer_controller))
  (`/Engine/EditorBlueprintResources/StandardMacros.IsValid` _returnvalue
    (:`Is Valid`
      (`EnhancedInputSubsystemInterface.AddMappingContext` _returnvalue "/Game/Characters/Input/IMC_Default.IMC_Default" 0 (struct)))))

(event `EnhancedInput|/Game/Characters/Input/IA_Move`
  (params (ActionValue :type "Vector2D Structure") (ElapsedSeconds :type "Float (double-precision)") (TriggeredSeconds :type "Float (double-precision)") (InputAction :type "InputAction Object Reference" :default "/Game/Characters/Input/IA_Move.IA_Move"))
  (:`Triggered`
    (set `self.Delta Rotation Z (Yaw)` ActionValue_X))
  (:`Completed`
    (set `self.Delta Rotation Z (Yaw)` 0.0)))

(event `EnhancedInput|/Game/Characters/Input/IA_Look`
  (params (ActionValue :type "Vector2D Structure") (ElapsedSeconds :type "Float (double-precision)") (TriggeredSeconds :type "Float (double-precision)") (InputAction :type "InputAction Object Reference" :default "/Game/Characters/Input/IA_Look.IA_Look"))
  (:`Triggered`
    (`self.AddControllerYawInput` ActionValue_X)))

(fn `UserConstructionScript`)